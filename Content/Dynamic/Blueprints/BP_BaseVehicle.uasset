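; Base physics vehicle Blueprint built around a Body, a DriveComponent and four corner suspension components.
; Each tick it prints drive telemetry and eases spring arm rotation lag toward a looser value while the DriveComponent reports drifting.
; Debug keys cycle cameras, boost, toggle slow motion and suspension lines, and reset the body to its spawn location through ATP (async tick physics) calls.
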(event Custom|UpdateCameraRotationLag
  ;[1 1 1 1 98] CameraStuff
  (bind _returnvalue (Class|DriveComponent|GetDriftingState (Variables|Default|GetDriveComponent)))
  (if _returnvalue
    (Variables|/Script/Engine.SpringArmComponent|SetCameraRotationLagSpeed (Variables|Default|GetSpringArm) (Math|Interpolation|FInterpTo (Variables|/Script/Engine.SpringArmComponent|GetCameraRotationLagSpeed (Variables|Default|GetSpringArm)) 2.0 (Utilities|Time|GetWorldDeltaSeconds) 12.0))
    (else
      (Variables|/Script/Engine.SpringArmComponent|SetCameraRotationLagSpeed (Variables|Default|GetSpringArm) (Math|Interpolation|FInterpTo (Variables|/Script/Engine.SpringArmComponent|GetCameraRotationLagSpeed (Variables|Default|GetSpringArm)) 1e+01 (Utilities|Time|GetWorldDeltaSeconds) 6.0)))))

(event EventBeginPlay
  (bind _returnvalue (Class|AsyncTickFunctions|ATPGetTransform (Variables|Default|GetBody)))
  (Variables|Default|SetSpawnTransform _returnvalue)
  (Development|PrintString (Utilities|GetDisplayName (Variables|/Script/ArcadeRacer.DriveComponent|GetParentVehicle (Variables|Default|GetDriveComponent))) true true "(R=1.000000,G=0.000000,B=0.413675,A=1.000000)")
  (Development|PrintString (Utilities|GetDisplayName (Variables|Default|GetBody)) true true "(R=0.242424,G=1.000000,B=0.000000,A=1.000000)"))

(event Collision|EventActorBeginOverlap
  (params (OtherActor :type Actor%20Object%20Reference)))

(event EventTick
  (params (DeltaSeconds :type Float%20%28single-precision%29))
  (bind _drivecomponent (Variables|Default|GetDriveComponent))
  (CallFunction|UpdateCameraRotationLag)
  (bind _returnvalue (Class|DriveComponent|GetLateralSpeedNormalized _drivecomponent))
  ;[0 0 0] Display Input
  (bind _returnvalue_2 (Class|DriveComponent|GetCurrentSpeed _drivecomponent))
  (Development|PrintString (Utilities|String|ToString(Text) (Utilities|Text|FormatText "Kmh: {fs} 
Drift Coef:{drift} 
Traction: {t} 
Accel multiplier: {am} 
 
Throttle Input: {ti} 
Steering Input: {si}" _returnvalue_2 _returnvalue (Variables|/Script/ArcadeRacer.DriveComponent|GetTractionMultiplier _drivecomponent) (Variables|/Script/ArcadeRacer.DriveComponent|GetAccelerationMultiplier _drivecomponent) (Variables|/Script/ArcadeRacer.DriveComponent|GetThrottleInput _drivecomponent) (Variables|/Script/ArcadeRacer.DriveComponent|GetSteeringInput _drivecomponent))) true true "(R=0.674632,G=1.000000,B=0.269644,A=1.000000)" 0.0))

(event Collision|EventHit
  (params (MyComp :type Primitive%20Component%20Object%20Reference) (Other :type Actor%20Object%20Reference) (OtherComp :type Primitive%20Component%20Object%20Reference) (bSelfMoved :type Boolean) (HitLocation :type Vector :default "0, 0, 0") (HitNormal :type Vector :default "0, 0, 0") (NormalImpulse :type Vector :default "0, 0, 0") (Hit :type Hit%20Result%20Structure%20%28by%20ref%29)))

(event Input|KeyboardEvents|X
  (params (Key :type Key%20Structure :default "None"))
  (:Pressed
    (Utilities|FlowControl|FlipFlop
      (:A
        (Utilities|Time|SetGlobalTimeDilation 0.1))
      (:B
        (Utilities|Time|SetGlobalTimeDilation 1.0)))))

(event Input|KeyboardEvents|V
  (params (Key :type Key%20Structure :default "None"))
  (bind _body (Variables|Default|GetBody))
  ;[0 0 0] Debug functions to be remoived
  ;;[0 0 0] Debug add impulse
  (:Pressed
    (bind _returnvalue (Class|DriveComponent|GetCurrentSpeed (Variables|Default|GetDriveComponent)))
    (if (< _returnvalue 1.1e+03)
      (Physics|AddImpulse _body (* (Math|Vector|GetForwardVector _body) 6e+06) "None" false))))

(event Input|KeyboardEvents|E
  (params (Key :type Key%20Structure :default "None"))
  (bind _debugsidecam (Variables|Default|GetDebugSideCam))
  (bind _fps (Variables|Default|GetFPS))
  (bind _camera (Variables|Default|GetCamera))
  (bind _array (Utilities|Array|MakeArray _camera _debugsidecam _fps))
  ;[0 0 0] Debug functions to be remoived
  ;;[0 0 0] DebugCamChange
  (:Pressed
    (Math|Integer|IncrementInt (Variables|Default|GetCameraIndex)
      (:%20%20
        (if (> (Variables|Default|GetCameraIndex) (- (Utilities|Array|Length _array) 1))
          (Variables|Default|SetCameraIndex 0))
        (for _array_element _array
          (Components|Activation|Deactivate _array_element))
        (Components|Activation|Activate (Utilities|Array|Get(acopy) _array (Variables|Default|GetCameraIndex)) false)))))

(event Input|KeyboardEvents|R
  (params (Key :type Key%20Structure :default "None"))
  (bind _body (Variables|Default|GetBody))
  ;[0 0 0] Debug functions to be remoived
  ;;[0 0 0] Placeholder reset
  (:Pressed
    (Class|AsyncTickFunctions|ATPSetWorldLocationandRotation (Variables|Default|GetBody) (.location (Variables|Default|GetSpawnTransform)) "90.000000,0.000000,0.000000")
    (Class|AsyncTickFunctions|ATPSetLinearVelocity _body "0, 0, 0" false "None")
    (Class|AsyncTickFunctions|ATPSetAngularVelocityinDegrees _body "0, 0, 0" false "None")))

(event Input|KeyboardEvents|0
  (params (Key :type Key%20Structure :default "None"))
  (bind _suspensionrr (Variables|Default|GetSuspensionRR))
  (bind _suspensionrl (Variables|Default|GetSuspensionRL))
  (bind _suspensionfl (Variables|Default|GetSuspensionFL))
  (bind _suspensionfr (Variables|Default|GetSuspensionFR))
  ;[0 0 0] Debug functions to be remoived
  (:Pressed
    (Variables|/Script/ArcadeRacer.SuspensionComponent|SetDrawDebugLines _suspensionrr (not (Variables|/Script/ArcadeRacer.SuspensionComponent|GetDrawDebugLines _suspensionrr)))
    (Variables|/Script/ArcadeRacer.SuspensionComponent|SetDrawDebugLines _suspensionrl (not (Variables|/Script/ArcadeRacer.SuspensionComponent|GetDrawDebugLines _suspensionrl)))
    (Variables|/Script/ArcadeRacer.SuspensionComponent|SetDrawDebugLines _suspensionfl (not (Variables|/Script/ArcadeRacer.SuspensionComponent|GetDrawDebugLines _suspensionfl)))
    (Variables|/Script/ArcadeRacer.SuspensionComponent|SetDrawDebugLines _suspensionfr (not (Variables|/Script/ArcadeRacer.SuspensionComponent|GetDrawDebugLines _suspensionfr)))))

(event Input|KeyboardEvents|P
  (params (Key :type Key%20Structure :default "None"))
  (:Pressed
    (Development|PrintString (Utilities|String|ToString(Float) (Variables|/Script/ArcadeRacer.SuspensionComponent|GetWheelRadius (Variables|Default|GetSuspensionFL))))))

(fn ConstructionScript)